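; RTS-style player controller that handles unit selection, move orders, camera look, HUD, menus and game speed.
; Left click traces, or drag box screen-projects, to select pawns, flagging their PlayerAI and spawning markers.
; Right-drag rotates the camera, while a right click, detected by unchanged control rotation, pushes MoveTo actions offset from the group's center to keep formation.
; It creates overlay widgets, swaps one modal widget, and routes pause and time dilation to GM_SpaceTroopers.
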(event `VisualizeAction`
  (params (Location :type "Vector Structure") (Action :type "/Game/Gameplay/Player/EAction Enum" :default "NewEnumerator0"))
  (switch `/Game/Gameplay/Player/EAction` Action
    (:`NewEnumerator0`
      (`GameplayStatics.PlaySound2D` "/Game/Audio/UI/NotSelected.NotSelected" 1.0 1.0 0.0 null null))
    (:`NewEnumerator1`
      (`GameplayStatics.PlaySound2D` "/Game/Audio/UI/Acknowledge.Acknowledge" 1.0 1.0 0.0 null null)))
  (`self.SpawnCircle` Location))

(event `AddPawnToSelection`
  (params (Pawn :type "Pawn Object Reference"))
  (bind _selectedpawns (`self.SelectedPawns`))
  (`/Engine/EditorBlueprintResources/StandardMacros.IsValid` Pawn
    (:`Is Valid`
      (if (not (`KismetArrayLibrary.Array_Contains` _selectedpawns Pawn))
        (`KismetArrayLibrary.Array_Add` _selectedpawns Pawn)
        (`|ExecutionSequence`
          (:`then_0`
            (bind _asplayer_ai (cast `/Game/Gameplay/AI/PlayerAI` (`AIBlueprintHelperLibrary.GetAIController` Pawn)))
            (`/Game/Gameplay/AI/PlayerAI.SetSelected` _asplayer_ai true))
          (:`then_1`
            (bind _returnvalue (`|SpawnActorFromClass` "/Game/Gameplay/Player/SelectionMarker.SelectionMarker_C" (`KismetMathLibrary.Conv_VectorToTransform` (`self.K2_GetActorLocation` Pawn)) "AlwaysSpawn" "OverrideRootScale" null Pawn 0.0 true null))
            (`KismetArrayLibrary.Array_Add` (`self.Markers`) _returnvalue)))))))

(event `self.ReceiveBeginPlay`
  (`|ExecutionSequence`
    (:`then_0`
      (bind _returnvalue (`|CreateWidget` "/Game/Interface/PlayerHUD.PlayerHUD_C" self))
      (set `self.Hud` _returnvalue)
      (`UserWidget.AddToViewport` _returnvalue 0))
    (:`then_1`
      (set `self.bShowMouseCursor` true)
      (`WidgetBlueprintLibrary.SetInputMode_GameAndUIEx` self _returnvalue "LockOnCapture" false)
      (`GameplayStatics.SetViewportMouseCaptureMode` "CapturePermanently_IncludingInitialMouseDown"))
    (:`then_2`
      (bind _returnvalue_2 (`|CreateWidget` "/Game/Interface/SelectionBox.SelectionBox_C" self))
      (set `self.SelectionBox` _returnvalue_2)
      (`UserWidget.AddToViewport` _returnvalue_2 0))
    (:`then_3`
      (bind _returnvalue_3 (`|CreateWidget` "/Game/Interface/ScreenFade.ScreenFade_C" self))
      (set `self.Fade` _returnvalue_3)
      (`UserWidget.AddToViewport` _returnvalue_3 0))
    (:`then_4`
      (bind _returnvalue_4 (`|CreateWidget` "/Game/Interface/Announcement.Announcement_C" self))
      (set `self.Announcement` _returnvalue_4)
      (`UserWidget.AddToViewport` _returnvalue_4 0))))

(event `FadeToBlack`
  (params (TransitionTime :type "Float (double-precision)"))
  (bind _fade (`self.Fade`)
    (:`then`
      (`/Game/Interface/ScreenFade.ToBlack` _fade TransitionTime))
    (:`else`)))

(event `FadeFromBlack`
  (params (TransitionTime :type "Float (double-precision)"))
  (bind _fade (`self.Fade`)
    (:`then`
      (`/Game/Interface/ScreenFade.FromBlack` _fade TransitionTime))
    (:`else`)))

(event `SetLookMode`
  (params (Enabled :type Boolean))
  (bind (_locationx _locationy) (`self.GetMousePosition`))
  (bind (_x _y) (`KismetMathLibrary.BreakVector2D` (`self.MousePosition`)))
  ;[1 1 1] Mouse move
  (if Enabled
    (set `self.bShowMouseCursor` false)
    (`WidgetBlueprintLibrary.SetInputMode_GameOnly` self)
    (set `self.MousePosition` (`KismetMathLibrary.MakeVector2D` _locationx _locationy))
    (else
      (set `self.bShowMouseCursor` true)
      (`WidgetBlueprintLibrary.SetInputMode_GameAndUIEx` self (`self.Hud`) "DoNotLock" false)
      (`self.SetMouseLocation` (`KismetMathLibrary.FTrunc` _x) (`KismetMathLibrary.FTrunc` _y)))))

(event `SelectMultiple`)

(event `SetViewportWIdget`
  (params (NewWidget :type "UserWidget Object Reference"))
  ;[1 1 1] Widgets
  (`/Engine/EditorBlueprintResources/StandardMacros.IsValid` NewWidget
    (:`Is Valid`
      (bind _currentwidget (`self.CurrentWidget`)
        (:`then`
          (if (not (== _currentwidget NewWidget))
            (`self.RemoveViewportWidget` :!label _label)
            (bind _output_get (set `self.CurrentWidget` NewWidget))
            (`UserWidget.AddToViewport` _output_get 0)))
        (:`else`
          (goto _label))))
    (:`Is Not Valid`
      (`self.RemoveViewportWidget`))))

(event `InputAction|Click`
  (params (Key :type "Key Structure"))
  (bind _selectionbox (`self.SelectionBox`))
  ;[1 1 1] Input
  (:`Pressed`
    (`self.IsClickAllowed`
      (:`Click`
        (`/Game/Interface/SelectionBox.StartCapture` _selectionbox))))
  (:`Released`
    (bind (_pos _size) (`/Game/Interface/SelectionBox.StopCapture` _selectionbox))
    (`self.IsClickAllowed`
      (:`Click`
        (`self.ClearSelection`)
        (if (`self.IsBigEnough` _size)
          (`self.SelectPawnsInBox` _pos _size)
          (if (`KismetArrayLibrary.Array_IsValidIndex` (`self.SelectedPawns`))
            (`GameplayStatics.PlaySound2D` "/Game/Audio/UI/Select.Select" 1.0 1.0 0.0 null null :!label _label_2)
            (else
              (`GameplayStatics.PlaySound2D` "/Game/Audio/UI/NotSelected.NotSelected" 1.0 1.0 0.0 null null)))
          (else
            (bind (_clickedpawn _clicklocation) (`self.GetClickLocation`))
            (`self.AddPawnToSelection` _clickedpawn)
            (`/Engine/EditorBlueprintResources/StandardMacros.IsValid` _clickedpawn
              (:`Is Valid`
                (goto _label_2))
              (:`Is Not Valid`
                (`self.VisualizeAction` _clicklocation)))))))))

(event `InputAxis|CameraPitch`
  (params (AxisValue :type "Float (single-precision)"))
  ;[1 1 1] Mouse move
  (if (`self.IsInputKeyDown` "RightMouseButton")
    (`self.AddPitchInput` (* AxisValue -1.0))))

(event `RemoveViewportWidget`
  ;[1 1 1] Widgets
  (bind _currentwidget (`self.CurrentWidget`)
    (:`then`
      (`Widget.RemoveFromParent` _currentwidget)
      (set `self.CurrentWidget` null))
    (:`else`)))

(event `InputAxis|CameraYaw`
  (params (AxisValue :type "Float (single-precision)"))
  ;[1 1 1] Mouse move
  (if (`self.IsInputKeyDown` "RightMouseButton")
    (`self.AddYawInput` AxisValue)))

(event `RemoveWIdgetFromViewport`
  (params (TargetWidget :type "UserWidget Object Reference"))
  ;[1 1 1] Widgets
  (if (== TargetWidget (`self.CurrentWidget`))
    (`self.RemoveViewportWidget`)))

(event `InputAction|RightClick`
  (params (Key :type "Key Structure"))
  ;[1 1 1] Input
  (:`Pressed`
    (`self.SetLookMode` true)
    (`self.MouseCheck` 1.0 :!label _label_3
      (:`Click`
        (`self.IsClickAllowed`
          (:`Click`
            (`self.PushMoveToCommands`))))))
  (:`Released`
    (`self.SetLookMode` false)
    (goto _label_3 :!via `Release`)))

(event `ShowHelp`
  (bind _helpwidget (`self.HelpWidget`))
  ;[1 1 1] Input
  (`/Engine/EditorBlueprintResources/StandardMacros.IsValid` (`self.HelpWidget`) :!label _label_4
    (:`Is Valid`
      _)
    (:`Is Not Valid`
      (bind _returnvalue (`|CreateWidget` "/Game/Interface/Help.Help_C" self))
      (bind _output_get (set `self.HelpWidget` _returnvalue))))
  (if (`Widget.IsInViewport` _output_get)
    (`self.RemoveWIdgetFromViewport` _helpwidget)
    (else
      (`self.SetViewportWIdget` _helpwidget))))

(event `InputAction|Help`
  (params (Key :type "Key Structure"))
  ;[1 1 1] Input
  (:`Released`
    (goto _label_4)))

(event `ShowMenu`
  (bind _menuwidget (`self.MenuWIdget`))
  (bind _asgm_space_troopers (cast `/Game/Gameplay/GM_SpaceTroopers` (`GameplayStatics.GetGameMode`) :!pure true))
  ;[1 1 1] Input
  (`/Engine/EditorBlueprintResources/StandardMacros.IsValid` (`self.MenuWIdget`) :!label _label_5
    (:`Is Valid`
      _)
    (:`Is Not Valid`
      (bind _returnvalue (`|CreateWidget` "/Game/Interface/Menu.Menu_C" self))
      (bind _output_get (set `self.MenuWIdget` _returnvalue))))
  (if (`Widget.IsInViewport` _output_get)
    (`self.RemoveWIdgetFromViewport` _menuwidget :!label _label_6)
    (`/Game/Gameplay/GM_SpaceTroopers.SetPaused` _asgm_space_troopers false)
    (else
      (`self.SetViewportWIdget` _menuwidget)
      (`/Game/Gameplay/GM_SpaceTroopers.SetPaused` _asgm_space_troopers true))))

(event `CloseMenu`
  ;[1 1 1] Input
  (goto _label_6))

(event `InputAction|Menu`
  (params (Key :type "Key Structure"))
  ;[1 1 1] Input
  (:`Released`
    (goto _label_5)))

(event `InputAction|Pause`
  (params (Key :type "Key Structure"))
  ;[1 1 1] Input
  (:`Released`
    (bind _asgm_space_troopers (cast `/Game/Gameplay/GM_SpaceTroopers` (`GameplayStatics.GetGameMode`)))
    (`/Game/Gameplay/GM_SpaceTroopers.SetPaused` _asgm_space_troopers (not (`/Game/Gameplay/GM_SpaceTroopers.IsPaused` _asgm_space_troopers)))))

(event `InputAction|SlowDown`
  (params (Key :type "Key Structure"))
  ;[1 1 1] Input
  (:`Released`
    (bind _asgm_space_troopers (cast `/Game/Gameplay/GM_SpaceTroopers` (`GameplayStatics.GetGameMode`)))
    (`/Game/Gameplay/GM_SpaceTroopers.DecreaseDilation` _asgm_space_troopers)))

(event `InputAction|SpeedUp`
  (params (Key :type "Key Structure"))
  ;[1 1 1] Input
  (:`Released`
    (bind _asgm_space_troopers (cast `/Game/Gameplay/GM_SpaceTroopers` (`GameplayStatics.GetGameMode`)))
    (`/Game/Gameplay/GM_SpaceTroopers.IncreaseDilation` _asgm_space_troopers)))

(fn `ClearSelection`
  (bind _selectedpawns (`self.SelectedPawns`))
  (bind _markers (`self.Markers`))
  (for _array_element _selectedpawns
    (bind _asplayer_ai (cast `/Game/Gameplay/AI/PlayerAI` (`AIBlueprintHelperLibrary.GetAIController` _array_element)))
    (`/Game/Gameplay/AI/PlayerAI.SetSelected` _asplayer_ai false))
  (`KismetArrayLibrary.Array_Clear` _selectedpawns)
  (for _array_element_2 _markers
    (`/Engine/EditorBlueprintResources/StandardMacros.IsValid` _array_element_2
      (:`Is Valid`
        (`self.K2_DestroyActor` _array_element_2))))
  (`KismetArrayLibrary.Array_Clear` _markers))

(fn `GetClickLocation`
  (returns (ClickedPawn :type "Pawn Object Reference") (ClickLocation :type "Vector Structure"))
  (locals (ClickLoc :type "Vector Structure" :default (0.0 0.0 0.0)))
  (bind (_worldlocation _worlddirection) (`self.DeprojectMousePositionToWorld`))
  (bind _clickloc (`local.ClickLoc`))
  (set `local.ClickLoc` (`/Game/Utility/UtilityFunctiuons.IntersectLayer` _worldlocation _worlddirection))
  (bind _outhit (`KismetSystemLibrary.LineTraceSingleForObjects` _worldlocation (+ _worldlocation (* _worlddirection 10000.0)) (`|MakeArray` "ObjectTypeQuery3" :!type "EObjectTypeQuery Enum") true))
  (bind _aspawn (cast `Pawn` (`.HitActor` (`GameplayStatics.BreakHitResult` _outhit)))
    (:`then`
      (return _aspawn _clickloc))
    (:`CastFailed`
      (return null _clickloc))))

(fn `GetSelectedController`
  (returns (`AsAI Base` :type "/Game/Gameplay/AI/PlayerAI Object Reference"))
  (bind _selectedpawn (`self.SelectedPawn`)
    (:`then`
      (bind _asplayer_ai (cast `/Game/Gameplay/AI/PlayerAI` (`AIBlueprintHelperLibrary.GetAIController` _selectedpawn))
        (:`then`
          (return _asplayer_ai))
        (:`CastFailed`
          _)))
    (:`else`
      _))
  (return null))

(fn `PushMoveToCommands`
  (locals (Offset :type "Vector Structure" :default (0.0 0.0 0.0)))
  (if (`KismetArrayLibrary.Array_IsValidIndex` (`self.SelectedPawns`))
    (`|ExecutionSequence`
      (:`then_0`
        (bind (_clickedpawn _clicklocation) (`self.GetClickLocation`))
        (`self.VisualizeAction` _clicklocation "NewEnumerator1")
        (bind _center (`GameplayStatics.GetActorArrayBounds` (`self.SelectedPawns`) true))
        (set `local.Offset` (* (- _clicklocation _center) (1.0 1.0 0.0))))
      (:`then_1`
        (for _array_element (`self.SelectedPawns`)
          (bind _asplayer_ai (cast `/Game/Gameplay/AI/PlayerAI` (`AIBlueprintHelperLibrary.GetAIController` _array_element)))
          (bind _returnvalue (`|GenericCreateObject` "/Game/Gameplay/AI/Actions/AI_Action_MoveTo.AI_Action_MoveTo_C" _asplayer_ai (+ (`local.Offset`) (`self.K2_GetActorLocation` (`self.K2_GetPawn` _asplayer_ai))) 50.0 5.0))
          (`/Game/Gameplay/AI/PlayerAI.PushAction` _asplayer_ai _returnvalue))))))

(fn `SelectPawnsInBox`
  (params (BoxPos :type "Vector2D Structure") (BoxSize :type "Vector2D Structure"))
  (locals (ProjectedLoc :type "Vector2D Structure") (Selected :type "Array of /Game/Gameplay/AI/CommandablePawn Object Reference"))
  (bind _boxpos (`local.BoxPos`))
  (bind (_x _y) (`KismetMathLibrary.BreakVector2D` _boxpos))
  (bind (_x_2 _y_2) (`KismetMathLibrary.BreakVector2D` (+ _boxpos (`local.BoxSize`))))
  (bind _outactors (`GameplayStatics.GetAllActorsOfClass` "/Game/Gameplay/AI/CommandablePawn.CommandablePawn_C"))
  (for _array_element _outactors
    (cast `/Game/Gameplay/Troops/Ship` _array_element)
    (if (`|EnumEquality` (`/Game/Gameplay/AI/CommandablePawn.Team` _array_element) "NewEnumerator1")
      (bind (_screenlocation _returnvalue) (`self.ProjectWorldLocationToScreen` (`self.K2_GetActorLocation` _array_element)))
      (if _returnvalue
        (bind _output_get (set `local.ProjectedLoc` _screenlocation))
        (bind (_x_3 _y_3) (`KismetMathLibrary.BreakVector2D` _output_get))
        (if (and (> _x_3 _x) (> _y_3 _y) (< _x_3 _x_2) (< _y_3 _y_2))
          (`self.AddPawnToSelection` _array_element))))))

(fn `SpawnCircle`
  (params (Location :type "Vector Structure") (Color :type "LinearColor Structure"))
  (`|SpawnActorFromClass` "/Game/Gameplay/Player/ClickActor.ClickActor_C" (`KismetMathLibrary.MakeTransform` Location) "Undefined" "OverrideRootScale" null Color null))

(fn `UserConstructionScript`)