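; Player controller for the Space Troopers game that shows the mouse cursor and adds the player HUD on begin play.
; On a Click press it deprojects the mouse position, intersects that ray with a layer, and spawns a click particle effect at the hit point.
; The effect's custom time dilation comes from the game mode's realtime dilation value.
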(event `self.ReceiveBeginPlay`
  (set `self.bShowMouseCursor` true)
  (bind _returnvalue (`|CreateWidget` "/Game/Interface/PlayerHUD.PlayerHUD_C" self))
  (`UserWidget.AddToViewport` _returnvalue 0))

(event `InputAction|Click`
  (params (Key :type "Key Structure"))
  (bind (_worldlocation _worlddirection) (`self.DeprojectMousePositionToWorld`))
  (:`Pressed`
    (bind _returnvalue (`GameplayStatics.SpawnEmitterAtLocation` "/Game/VFX/Click.Click" (`/Game/Utility/UtilityFunctiuons.IntersectLayer` _worldlocation _worlddirection)))
    (set `ParticleSystemComponent.CustomTimeDilation` (`/Game/Gameplay/GM_SpaceTroopers.GetRealtimeDilation` (cast `/Game/Gameplay/GM_SpaceTroopers` (`GameplayStatics.GetGameMode`) :!pure true)) _returnvalue)))

(fn `UserConstructionScript`)