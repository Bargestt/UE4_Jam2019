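; Game mode for SpaceTroopers that runs level flow from startup menu through intro to Round1 and controls game speed and pause.
; Levels swap as streaming levels, destroying projectiles, troops and AI controllers, then moving the PlayerCamera to a PlayerStart.
; Camera input and click permission are restricted during menu and intro.
; Pause and speed steps use global time dilation, with inverse CustomTimeDilation keeping player controller and pawn at real-time speed.
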(event `IncreaseDilation`
  (bind _returnvalue (`GameplayStatics.GetPlayerController` 0))
  (bind _returnvalue_2 (`self.GetRealtimeDilation`))
  (`GameplayStatics.SetGlobalTimeDilation` (`KismetMathLibrary.FClamp` (+ (`GameplayStatics.GetGlobalTimeDilation`) (`self.DialtionStep`))))
  (`self.OnDilationChanged` :!label _label)
  (set `Actor.CustomTimeDilation` _returnvalue_2 _returnvalue)
  (set `Actor.CustomTimeDilation` _returnvalue_2 (`Controller.K2_GetPawn` _returnvalue)))

(event `DecreaseDilation`
  (`GameplayStatics.SetGlobalTimeDilation` (`KismetMathLibrary.FClamp` (- (`GameplayStatics.GetGlobalTimeDilation`) (`self.DialtionStep`))))
  (goto _label))

(event `SetPaused`
  (params (Paused :type Boolean))
  (`GameplayStatics.SetGlobalTimeDilation` (select `bool` Paused :`false` 1.0 :!type "Float (single-precision)"))
  (goto _label))

(event `FindAndSetRestricted`
  (params (IsRestricted :type Boolean))
  (bind _outactors (`GameplayStatics.GetAllActorsOfClass` "/Game/Gameplay/Player/PlayerCamera.PlayerCamera_C"))
  (bind _first (`/Game/Utility/UtilityMacro.GetFIrst` _outactors)
    (:`HasFirst`
      (`self.RestrictCamera` _first IsRestricted))))

(event `RestrictCamera`
  (params (Target :type "/Game/Gameplay/Player/PlayerCamera Object Reference") (IsRestricted :type Boolean))
  (bind _returnvalue (not IsRestricted))
  (`/Game/Gameplay/Player/PlayerCamera.SetAllowInput` Target _returnvalue)
  (bind _asplayer_controller_bp (cast `/Game/Gameplay/Player/PlayerControllerBP` (`Pawn.GetController` Target)))
  (set `/Game/Gameplay/Player/PlayerControllerBP.AllowClick` _returnvalue _asplayer_controller_bp))

(event `MainMenu`
  (`self.LoadLevel` "StartupMap"))

(event `self.ReceiveBeginPlay`
  (`/Engine/EditorBlueprintResources/StandardMacros.IsValid` (`GameplayStatics.GetStreamingLevel` "StartupMap")
    (:`Is Valid`
      (`self.LoadLevel` "StartupMap")
      (bind _asplayer_controller_bp (cast `/Game/Gameplay/Player/PlayerControllerBP` (`GameplayStatics.GetPlayerController` 0)))
      (`/Game/Gameplay/Player/PlayerControllerBP.ShowMenu` _asplayer_controller_bp)
      (`self.SetPaused` false))))

(event `NewGame`
  (`self.LoadLevel` "IntroMap")
  (`self.FindAndSetRestricted` true)
  (`|ExecutionSequence`
    (:`then_0`
      (bind _returnvalue (`|CreateWidget` "/Game/Maps/Sequence/Intro.Intro_C" (`GameplayStatics.GetPlayerController` 0)))
      (`UserWidget.AddToViewport` _returnvalue 0)
      (add `/Game/Maps/Sequence/Intro.OnFinished` _returnvalue (delegate `OnFinished_Event_0`)))))

(event `LoadLevel`
  (params (PackageName :type Name))
  (`GameplayStatics.UnloadStreamLevel` (`self.Current`))
  (`self.Cleanup`)
  (bind _output_get (set `self.Current` PackageName))
  (`GameplayStatics.LoadStreamLevel` _output_get true)
  (`|ExecutionSequence`
    (:`then_0`
      ;[1 1 1] Move camera
      (bind _outactors (`GameplayStatics.GetAllActorsOfClass` "/Script/Engine.PlayerStart"))
      (bind _first (`/Game/Utility/UtilityMacro.GetFIrst` _outactors)
        (:`HasFirst`
          (bind _outactors_2 (`GameplayStatics.GetAllActorsOfClass` "/Game/Gameplay/Player/PlayerCamera.PlayerCamera_C"))
          (bind _first_2 (`/Game/Utility/UtilityMacro.GetFIrst` _outactors_2)
            (:`HasFirst`
              (`self.RestrictCamera` _first_2 (== (`self.Current`) (`self.MainMenuMap`)))
              (`self.K2_SetActorTransform` _first_2 (`self.GetTransform` _first) false true)
              (`Controller.SetControlRotation` (`Pawn.GetController` _first_2) (`self.K2_GetActorRotation` _first)))))))))

(event `OnFinished_Event_0`
  (`self.LoadLevel` "Round1")
  (bind _outactors (`GameplayStatics.GetAllActorsOfClass` "/Game/Gameplay/Player/PlayerCamera.PlayerCamera_C"))
  (bind _first (`/Game/Utility/UtilityMacro.GetFIrst` _outactors)
    (:`HasFirst`
      (`self.RestrictCamera` _first)
      (`PlayerController.SetViewTargetWithBlend` (`GameplayStatics.GetPlayerController` 0) _first 0.0 "VTBlend_Linear" 0.0 false))))

(event `Cleanup`
  (`self.DeleteAll` "/Game/Gameplay/Weapons/Projectile.Projectile_C")
  (`self.DeleteAll` "/Game/Gameplay/Troops/BasicTroop.BasicTroop_C")
  (`self.DeleteAll` "/Script/AIModule.AIController"))

(event `TroopSpawned`
  (params (Troop :type "/Game/Gameplay/Troops/BasicTroop Object Reference")))

(fn `DeleteAll`
  (params (ActorClass :type "Actor Class Reference"))
  (bind _outactors (`GameplayStatics.GetAllActorsOfClass` ActorClass))
  (for _array_element _outactors
    (`self.K2_DestroyActor` _array_element)))

(fn `GetDilationPercent`
  (returns (Percent :type "Float (double-precision)"))
  (return (`GameplayStatics.GetGlobalTimeDilation`)))

(fn `GetRealtimeDilation`
  (returns (ReturnValue :type "Float (double-precision)"))
  (return (/ 1.0 (`GameplayStatics.GetGlobalTimeDilation`))))

(fn `IsPaused`
  (returns (IsPaused :type Boolean))
  (return (<= (`GameplayStatics.GetGlobalTimeDilation`) 0.01)))

(fn `IsStartupMap`
  (returns (ReturnValue :type Boolean))
  (return (== (`self.Current`) "StartupMap")))

(fn `UserConstructionScript`)